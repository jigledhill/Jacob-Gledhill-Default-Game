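; Player pawn for a shooter with switchable rifle, shotgun and sniper loadouts, speed, damage and half-damage perks, and scoring for hits on players.
; Gun events set shared stats that drive CreateBulletLine, an authority-only spread line trace from the third-person camera that applies damage and spawns bullets.
; A Tick-fed gate repeats automatic fire.
; Death drops a marker, then teleports the pawn to a random PlayerStart with full health instead of destroying it.
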(event `self.ReceiveTick`
  (params (DeltaSeconds :type "Float (single-precision)"))
  ;[1 1 1] Ticks
  (`self.Gun_Auto_Tick`))

(event `Respawn`
  ;[1 1 1] Respawn
  ;;[1 1 1] Select Random SpawnPoint
  (bind _outactors (`GameplayStatics.GetAllActorsOfClass` "/Script/Engine.PlayerStart"))
  (bind _random_array_element (`self.Random_Array` _outactors))
  (set `self.Spawn_Transform` (`self.GetTransform` _random_array_element))
  (bind (_returnvalue_location _returnvalue_rotation) (`KismetMathLibrary.BreakTransform` (`self.GetTransform` _random_array_element)))
  ;;[1 1 1] Use in place of destroy
  (`self.K2_TeleportTo` _returnvalue_location _returnvalue_rotation)
  (`self.Reset Health`))

(event `Reset Health`
  ;[1 1 1] Respawn
  ;;[1 1 1] Reset Health to owning client
  (set `self.Health` (`self.Max_Health`)))

(event `Reset Guns For Perks`
  ;[1 1 1] Respawn
  ;;[1 1 1] Resets gun stats back to default before re applying perks
  (switch `int` (`self.Gun_Queue`)
    (:`0`
      (`self.PeaShooter`))
    (:`1`
      (`self.Rifle`))
    (:`2`
      (`self.Shotgun`))
    (:`3`
      (`self.Sniper`))))

(event `self.ReceiveBeginPlay`
  (`self.Rifle`))

(event `Key|M`
  (params (Key :type "Key Structure"))
  ;[1 1 1] Respawn
  ;;[1 1 1] Kill Self
  (:`Pressed`
    (set `self.Points` (- (`self.Points`) 100.0))
    (`self.Respawn`)))

(event `Reset Guns`
  ;[1 1 1] Respawn
  ;;[1 1 1] Reset Perks and guns every respawn
  (`SceneComponent.SetVisibility` (`self.Mesh_PeaShooter`) false true)
  (`SceneComponent.SetVisibility` (`self.Mesh_Sniper`) false true)
  (`SceneComponent.SetVisibility` (`self.Mesh_Rifle`) false true))

(event `Reset Perks`
  ;[1 1 1] Respawn
  ;;[1 1 1] Reset Perks and guns every respawn
  (set `self.Damage_Halfed?` false)
  (bind _output_get (set `self.Move_Speed` 800.0))
  (set `CharacterMovementComponent.MaxWalkSpeed` _output_get (`self.CharacterMovement`))
  (`self.Reset Guns For Perks`))

(event `InputAxis|Forward_Backward`
  (params (AxisValue :type "Float (single-precision)"))
  ;[1 1 1] This is all basic movement, no need to protect from cheats
  ;;[1 1 1] Movement
  (`self.AddMovementInput` (`KismetMathLibrary.GetForwardVector` (`KismetMathLibrary.MakeRotator` 0.0 0.0 (.yaw (`self.GetControlRotation`)))) AxisValue))

(event `Aiming`
  ;[1 1 1] This is all basic movement, no need to protect from cheats
  ;;[1 1 1] Change Speed when aiming
  (set `self.Anim_IsAiming` true)
  (set `CharacterMovementComponent.MaxWalkSpeed` (/ (`self.Move_Speed`) 4.0) (`self.CharacterMovement`))
  (`self.Start Zoom`))

(event `Start Zoom`
  ;[1 1 1] This is all basic movement, no need to protect from cheats
  ;;[1 1 1] Zoom camera
  (`CameraComponent.SetFieldOfView` (`self.ThirdPersonCamera`) (`self.Gun_Zoom`)))

(event `Key|RightMouseButton`
  (params (Key :type "Key Structure"))
  ;[1 1 1] This is all basic movement, no need to protect from cheats
  ;;[1 1 1] Change Speed when aiming
  (:`Pressed`
    (`self.Aiming`))
  (:`Released`
    (`self.NotAiming`)))

(event `NotAiming`
  ;[1 1 1] This is all basic movement, no need to protect from cheats
  ;;[1 1 1] Change Speed when aiming
  (set `CharacterMovementComponent.MaxWalkSpeed` (`self.Move_Speed`) (`self.CharacterMovement`))
  (set `self.Anim_IsAiming` false)
  (`self.Stop Zoom`))

(event `Stop Zoom`
  ;[1 1 1] This is all basic movement, no need to protect from cheats
  ;;[1 1 1] Zoom camera
  (`CameraComponent.SetFieldOfView` (`self.ThirdPersonCamera`) 100.0))

(event `InputAxis|Left_Right`
  (params (AxisValue :type "Float (single-precision)"))
  ;[1 1 1] This is all basic movement, no need to protect from cheats
  ;;[1 1 1] Movement
  (`self.AddMovementInput` (`KismetMathLibrary.GetRightVector` (`self.GetControlRotation`)) AxisValue))

(event `Key|LeftMouseButton`
  (params (Key :type "Key Structure"))
  ;[1 1 1] Create Bullet
  (:`Pressed`
    (`self.Firing`))
  (:`Released`
    (`self.StopFiring`)))

(event `MakeGameHud`
  ;[1 1 1] This is all basic movement, no need to protect from cheats
  ;;[1 1 1] Show HUD
  (bind _returnvalue (`|CreateWidget` "/Game/BluePrints/Player_UI.Player_UI_C"))
  (set `/Game/BluePrints/Player_UI.Health_Bar` null _returnvalue)
  (`UserWidget.AddToViewport` _returnvalue 0))

(event `StopFiring`
  ;[1 1 1] Create Bullet
  ;;[1 1 1] If gun is auto, use tick to fire on repeat
  (goto _label :!via `Close`))

(event `Gun_Auto_Tick`
  ;[1 1 1] Create Bullet
  ;;[1 1 1] If gun is auto, use tick to fire on repeat
  (`/Engine/EditorBlueprintResources/StandardMacros.Gate` true :!label _label
    (:`Exit`
      (`self.CallCreateBullet` :!label _label_2)
      (set `self.Can_Fire` false)
      (`KismetSystemLibrary.Delay` (`self.Gun_FireRate`))
      (set `self.Can_Fire` true))))

(event `Firing`
  ;[1 1 1] Create Bullet
  ;;[1 1 1] If gun is auto, use tick to fire on repeat
  (if (`self.Gun_IsAuto`)
    (goto _label :!via `Open`)
    (else
      (goto _label_2))))

(event `Key|J`
  (params (Key :type "Key Structure"))
  ;[1 1 1] This is all basic movement, no need to protect from cheats
  ;;[1 1 1] Switch Camera Perspective
  (:`Pressed`
    (`/Engine/EditorBlueprintResources/StandardMacros.FlipFlop`
      (:`A`
        (`ActorComponent.SetActive` (`self.ThirdPersonCamera`) true false)
        (`ActorComponent.SetActive` (`self.FirstPersonCamera`) false true))
      (:`B`
        (`ActorComponent.SetActive` (`self.FirstPersonCamera`) true false)
        (`ActorComponent.SetActive` (`self.ThirdPersonCamera`) false true)))))

(event `CallCreateBullet`
  ;[1 1 1] Create Bullet
  (`self.CreateBulletLine`))

(event `InputAxis|Look_Left_Right`
  (params (AxisValue :type "Float (single-precision)"))
  ;[1 1 1] This is all basic movement, no need to protect from cheats
  ;;[1 1 1] Looking
  (`self.AddControllerYawInput` AxisValue))

(event `Jumping`
  ;[1 1 1] This is all basic movement, no need to protect from cheats
  ;;[1 1 1] Jumping
  (`/Engine/EditorBlueprintResources/ActorMacros.Switch Has Authority`
    (:`Authority`
      _)
    (:`Remote`
      _))
  (set `self.Anim_IsJumping` true)
  (`self.LaunchCharacter` (0.0 0.0 350.0))
  (`KismetSystemLibrary.Delay` 0.2)
  (set `self.Anim_IsJumping` false))

(event `Key|R`
  (params (Key :type "Key Structure"))
  ;[1 1 1] Create Bullet
  (:`Pressed`
    (`self.Reload`)))

(event `self.ReceiveAnyDamage`
  (params (Damage :type "Float (single-precision)") (DamageType :type "DamageType Object Reference") (InstigatedBy :type "Controller Object Reference") (DamageCauser :type "Actor Object Reference"))
  ;[1 1 1] Create Bullet
  (`self.RecieveDamage` Damage))

(event `InputAction|Jump`
  (params (Key :type "Key Structure"))
  ;[1 1 1] This is all basic movement, no need to protect from cheats
  ;;[1 1 1] Jumping
  (:`Pressed`
    (`self.Jumping`)))

(event `InputAxis|Look_Up_Down`
  (params (AxisValue :type "Float (single-precision)"))
  ;[1 1 1] This is all basic movement, no need to protect from cheats
  ;;[1 1 1] Looking
  (`self.AddControllerPitchInput` AxisValue))

(event `Reload`
  ;[1 1 1] Create Bullet
  (if (not (`self.Anim_IsReloading`))
    (set `self.Anim_IsReloading` true)
    (`KismetSystemLibrary.Delay` 2.0)
    (set `self.Gun_Clip` (`self.Gun_Max_Clip`))
    (set `self.Anim_IsReloading` false)))

(event `Gun_Sound`
  (params (Location :type "Vector Structure"))
  ;[1 1 1] Create Bullet
  (`GameplayStatics.PlaySoundAtLocation` "/Game/StarterContent/Audio/Explosion01.Explosion01" Location (struct) 0.5 1.0 0.0 null null null))

(event `PeaShooter`
  ;[1 1 1] PeaShooter
  (set `self.Gun_Clip` 1.0)
  (set `self.Gun_Max_Clip` 1.0)
  (set `self.Gun_Spread-` -0.001)
  (set `self.Gun_Spread+` 0.001)
  (set `self.Gun_BulletDamage` 1.0)
  (set `self.Gun_FireRate` 1.0)
  (set `self.Gun_Shots` 1.0)
  (set `self.Gun_IsAuto` false))

(event `Key|P`
  (params (Key :type "Key Structure"))
  (bind _returnvalue (`GameplayStatics.GetPlayerController` 0))
  ;[1 1 1] Create UI for class and perk change
  (:`Pressed`
    (bind _returnvalue_2 (`|CreateWidget` "/Game/BluePrints/Widgets/BP_Bonus_Select.BP_Bonus_Select_C" (`GameplayStatics.GetPlayerController` 0)))
    (`UserWidget.AddToViewport` _returnvalue_2 0)
    (`WidgetBlueprintLibrary.SetInputMode_UIOnlyEx` _returnvalue null)
    (set `PlayerController.bShowMouseCursor` true _returnvalue)))

(event `Rifle`
  ;[1 1 1] Rifle
  (set `self.Gun_Clip` 30.0)
  (set `self.Gun_Max_Clip` 30.0)
  (set `self.Gun_Spread-` -0.005)
  (set `self.Gun_Spread+` 0.005)
  (set `self.Gun_BulletDamage` 40.0)
  (set `self.Gun_FireRate` 0.15)
  (set `self.Gun_Shots` 1.0)
  (set `self.Gun_IsAuto` true)
  (set `self.Gun_Zoom` 50.0)
  (set `self.Gun_Queue` 1)
  (`SceneComponent.SetVisibility` (`self.Mesh_Rifle`) true true))

(event `Key|One`
  (params (Key :type "Key Structure"))
  ;[1 1 1] Workaround for perk selection UI
  (:`Pressed`
    (`self.Reset Guns`)
    (`self.Rifle`)
    (set `self.UI_Gun` "Assault Rifle")))

(event `Shotgun`
  ;[1 1 1] Shotgun
  (set `self.Gun_Clip` 8.0)
  (set `self.Gun_Max_Clip` 8.0)
  (set `self.Gun_Spread-` -0.05)
  (set `self.Gun_Spread+` 0.05)
  (set `self.Gun_BulletDamage` 12.0)
  (set `self.Gun_FireRate` 0.5)
  (set `self.Gun_Shots` 8.0)
  (set `self.Gun_IsAuto` false)
  (set `self.Gun_Zoom` 80.0)
  (set `self.Gun_Queue` 2)
  (`SceneComponent.SetVisibility` (`self.Mesh_PeaShooter`) true true))

(event `Key|Two`
  (params (Key :type "Key Structure"))
  ;[1 1 1] Workaround for perk selection UI
  (:`Pressed`
    (`self.Reset Guns`)
    (`self.Shotgun`)
    (set `self.UI_Gun` "Shotgun")))

(event `Sniper`
  ;[1 1 1] Sniper
  (set `self.Gun_Clip` 5.0)
  (set `self.Gun_Max_Clip` 5.0)
  (set `self.Gun_Spread-` 0.0)
  (set `self.Gun_Spread+` 0.0)
  (set `self.Gun_BulletDamage` 100.0)
  (set `self.Gun_FireRate` 2.0)
  (set `self.Gun_Shots` 1.0)
  (set `self.Gun_IsAuto` false)
  (set `self.Gun_Zoom` 20.0)
  (set `self.Gun_Queue` 3)
  (`SceneComponent.SetVisibility` (`self.Mesh_Sniper`) true true))

(event `Key|Three`
  (params (Key :type "Key Structure"))
  ;[1 1 1] Workaround for perk selection UI
  (:`Pressed`
    (`self.Reset Guns`)
    (`self.Sniper`)
    (set `self.UI_Gun` "Sniper Rifle")))

(event `Perk_Speed`
  ;[1 1 1] Speed Perk
  (bind _output_get (set `self.Move_Speed` (* (`self.Move_Speed`) 1.5)))
  (set `CharacterMovementComponent.MaxWalkSpeed` _output_get (`self.CharacterMovement`)))

(event `Key|Seven`
  (params (Key :type "Key Structure"))
  ;[1 1 1] Workaround for perk selection UI
  (:`Pressed`
    (`self.Reset Perks`)
    (`self.Perk_Speed`)
    (set `self.UI_Perk` "Speed Increase")))

(event `Key|Eight`
  (params (Key :type "Key Structure"))
  ;[1 1 1] Workaround for perk selection UI
  (:`Pressed`
    (`self.Reset Perks`)
    (`self.Perk_Damage`)
    (set `self.UI_Perk` "Deal Double Damage")))

(event `Perk_Damage`
  ;[1 1 1] Damage Perk
  (set `self.Gun_BulletDamage` (* (`self.Gun_BulletDamage`) 2.0)))

(event `Key|Nine`
  (params (Key :type "Key Structure"))
  ;[1 1 1] Workaround for perk selection UI
  (:`Pressed`
    (`self.Reset Perks`)
    (`self.Perk_Health`)
    (set `self.UI_Perk` "Recieve Half Damage")))

(event `Perk_Health`
  ;[1 1 1] Health Perk
  (set `self.Damage_Halfed?` true))

(fn `CreateBulletLine`
  (bind _gun_bulletdamage (`self.Gun_BulletDamage`))
  (bind _thirdpersoncamera (`self.ThirdPersonCamera`))
  (bind _returnvalue (`SceneComponent.K2_GetComponentLocation` _thirdpersoncamera))
  (bind _returnvalue_2 (`KismetMathLibrary.MakeVector` (+ (`KismetMathLibrary.RandomFloatInRange` (`self.Gun_Spread-`) (`self.Gun_Spread+`)) (.x (`SceneComponent.GetForwardVector` _thirdpersoncamera))) (+ (`KismetMathLibrary.RandomFloatInRange` (`self.Gun_Spread-`) (`self.Gun_Spread+`)) (.y (`SceneComponent.GetForwardVector` _thirdpersoncamera))) (+ (`KismetMathLibrary.RandomFloatInRange` (`self.Gun_Spread-`) (`self.Gun_Spread+`)) (.z (`SceneComponent.GetForwardVector` _thirdpersoncamera)))))
  (`/Engine/EditorBlueprintResources/ActorMacros.Switch Has Authority`
    (:`Authority`
      (if (`self.Anim_IsReloading`)
        _
        (elif (`self.Can_Fire`)
          ;[1 1 1] Check Ammo
          (if (> (`self.Gun_Clip`) 0.0)
            (`self.Gun_Sound` _returnvalue)
            ;[1 1 1] Bullets per shot
            (for _ (range (+ (`KismetMathLibrary.FTrunc` (- (`self.Gun_Shots`) 1.0)) 1))
              ;[1 1 1] Line Trace
              (bind _outhit (`KismetSystemLibrary.LineTraceSingle` _returnvalue (+ _returnvalue (* _returnvalue_2 1000000.0)) "TraceTypeQuery2"))
              (`GameplayStatics.ApplyDamage` (`.HitActor` (`GameplayStatics.BreakHitResult` _outhit)) _gun_bulletdamage (`self.GetInstigatorController`) self "/Script/Engine.DamageType")
              (`|SpawnActorFromClass` "/Game/Actors/Bullet.Bullet_C" (`KismetMathLibrary.MakeTransform` (`SceneComponent.K2_GetComponentLocation` (`self.BulletOrigin`)) (`KismetMathLibrary.Conv_VectorToRotator` _returnvalue_2)) "Undefined" "OverrideRootScale" null null)
              ;;[1 1 1] Only after hitting another player, add points and make particle effect
              (if (`ActorComponent.ComponentHasTag` (`.HitComponent` (`GameplayStatics.BreakHitResult` _outhit)) "Player")
                (`GameplayStatics.SpawnEmitterAtLocation` "/Game/StarterContent/Particles/P_Explosion.P_Explosion" (`.ImpactPoint` (`GameplayStatics.BreakHitResult` _outhit)) (struct) (0.1 0.1 0.1))
                (set `self.Points` (+ (`self.Points`) _gun_bulletdamage))))
            ;[1 1 1] Reduce clip after shot
            (set `self.Gun_Clip` (- (`self.Gun_Clip`) 1.0))
            (else
              ;[1 1 1] Reload
              (`self.Reload`))))))))

(fn `RecieveDamage`
  (params (damagepass :type "Float (double-precision)"))
  (if (`self.Damage_Halfed?`)
    (set `self.Health` (- (`self.Health`) (/ damagepass 2.0)))
    (else
      (set `self.Health` (- (`self.Health`) damagepass))))
  (if (<= (`self.Health`) 0.0)
    (`|SpawnActorFromClass` "/Game/BluePrints/BP_DeathMarker.BP_DeathMarker_C" (`KismetMathLibrary.Conv_VectorToTransform` (`KismetMathLibrary.TransformLocation` (`KismetMathLibrary.Conv_VectorToTransform` (`self.K2_GetActorLocation`)) (0.0 0.0 -85.0))) "AlwaysSpawn" "OverrideRootScale" null null)
    (`self.Respawn`)))

(fn `UserConstructionScript`)